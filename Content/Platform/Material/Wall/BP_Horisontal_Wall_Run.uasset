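; BP_Horisontal_Wall_Run is a wall platform Blueprint that tells overlapping actors when to start or stop a horizontal wall run.
; Two trigger components, H1 and H2, mark the ends of the run: entering either sends its transform as the start point and the other's location as the target.
; Leaving either trigger sends the same message without enabling it.
; A LeftOrRight flag, set only by H1, distinguishes the two ends.
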(event OnComponentBeginOverlap(h1)
  (params (OverlappedComponent :type Primitive%20Component%20Object%20Reference) (OtherActor :type Actor%20Object%20Reference) (OtherComp :type Primitive%20Component%20Object%20Reference) (OtherBodyIndex :type Integer) (bFromSweep :type Boolean) (SweepResult :type Hit%20Result%20Structure%20%28by%20ref%29))
  (Class|IBPWallRunVert|HorisontalWallRun(Message) OtherActor (Transformation|GetWorldLocation (Variables|Default|Geth2)) (Transformation|GetWorldTransform (Variables|Default|Geth1)) true true))

(event OnComponentEndOverlap(h1)
  (params (OverlappedComponent :type Primitive%20Component%20Object%20Reference) (OtherActor :type Actor%20Object%20Reference) (OtherComp :type Primitive%20Component%20Object%20Reference) (OtherBodyIndex :type Integer))
  (Class|IBPWallRunVert|HorisontalWallRun(Message) :self OtherActor :LeftOrRight true))

(event OnComponentBeginOverlap(h2)
  (params (OverlappedComponent :type Primitive%20Component%20Object%20Reference) (OtherActor :type Actor%20Object%20Reference) (OtherComp :type Primitive%20Component%20Object%20Reference) (OtherBodyIndex :type Integer) (bFromSweep :type Boolean) (SweepResult :type Hit%20Result%20Structure%20%28by%20ref%29))
  (Class|IBPWallRunVert|HorisontalWallRun(Message) OtherActor (Transformation|GetWorldLocation (Variables|Default|Geth1)) (Transformation|GetWorldTransform (Variables|Default|Geth2)) true false))

(event OnComponentEndOverlap(h2)
  (params (OverlappedComponent :type Primitive%20Component%20Object%20Reference) (OtherActor :type Actor%20Object%20Reference) (OtherComp :type Primitive%20Component%20Object%20Reference) (OtherBodyIndex :type Integer))
  (Class|IBPWallRunVert|HorisontalWallRun(Message) :self OtherActor))

(fn ConstructionScript)